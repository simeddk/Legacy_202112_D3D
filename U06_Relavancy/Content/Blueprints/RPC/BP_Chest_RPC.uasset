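; BP_Chest_RPC is a chest actor with a text label and a lid that toggles open and closed.
; The ToggleOpen event uses a FlipFlop to play or reverse a timeline that interpolates the Top component's relative rotation.
; The construction script applies the label text and creates a shared dynamic material instance for lid and base, driven by emissive color and intensity variables.
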(event Custom|ToggleOpen
  (Utilities|FlowControl|FlipFlop
    (:A
      (bind _alpha (Timeline|Timeline PlayFromStart)
        (:Update
          (Transformation|SetRelativeRotation (Variables|Default|GetTop) (Math|Rotator|Lerp(Rotator) "0, 0, 0" "130.000000, 0,0.000000" _alpha) false false))))
    (:B
      (Timeline|Timeline ReverseFromEnd))))

(fn ConstructionScript
  (CallFunction|SetMaterial)
  (Rendering|Components|TextRender|SetText (Variables|Default|GetTextRender) (Variables|Default|GetText)))

(fn SetMaterial
  (bind _returnvalue (Rendering|Material|CreateDynamicMaterialInstance "/Game/Objects/Chest/MAT_Chest_Inst.MAT_Chest_Inst" "None" :!class /Script/Engine.KismetMaterialLibrary))
  (Variables|Default|SetDynamicMaterial _returnvalue)
  (Rendering|Material|SetMaterial (Variables|Default|GetTop) 0 (Variables|Default|GetDynamicMaterial))
  (Rendering|Material|SetVectorParameterValue (Variables|Default|GetDynamicMaterial) "Emissive" (Variables|Default|GetEmissive) :!class /Script/Engine.MaterialInstanceDynamic)
  (Rendering|Material|SetScalarParameterValue (Variables|Default|GetDynamicMaterial) "Intensity" (Variables|Default|GetIntesity) :!class /Script/Engine.MaterialInstanceDynamic))