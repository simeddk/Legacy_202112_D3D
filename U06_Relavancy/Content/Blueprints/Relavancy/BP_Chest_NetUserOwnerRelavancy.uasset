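; Chest actor, named for net owner relevancy, that takes any overlapping actor as its owner and displays the owning player's name.
; On overlap by a ThirdPersonCharacter, the authority asks the client for the name in that character's NameWidget.
; The client returns it through a server call, which sets OwnerName, whose RepNotify updates OwnerNameText.
; Setting the owner first lets these calls route through the overlapping player's connection.
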(event OnComponentBeginOverlap(Box)
  (params (OverlappedComponent :type Primitive%20Component%20Object%20Reference) (OtherActor :type Actor%20Object%20Reference) (OtherComp :type Primitive%20Component%20Object%20Reference) (OtherBodyIndex :type Integer) (bFromSweep :type Boolean) (SweepResult :type Hit%20Result%20Structure%20%28by%20ref%29))
  (Actor|SetOwner OtherActor)
  (Networking|SwitchHasAuthority
    (:Authority
      (bind _asthird_person_character (Utilities|Casting|CastToThirdPersonCharacter OtherActor))
      (CallFunction|ClientGetText _asthird_person_character))))

(event Custom|Client_GetText
  (params (Player :type Third%20Person%20Character%20Object%20Reference))
  (CallFunction|ServerSetText (Class|TextBlock|GetText (Variables|/Game/Widgets/WB_Name.WB_Name_C|GetPlayerName (Variables|/Game/ThirdPersonBP/Blueprints/ThirdPersonCharacter.ThirdPersonCharacter_C|GetNameWidget Player)))))

(event Custom|Server_SetText
  (params (OwnerName :type Text))
  (Variables|Default|SetOwnerName OwnerName))

(fn ConstructionScript
  (|CallParentFunction))

(fn OnRepOwnerName
  (Rendering|Components|TextRender|SetText (Variables|Default|GetOwnerNameText) (Variables|Default|GetOwnerName)))