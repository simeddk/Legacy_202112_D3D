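; BP_RepNotify is a small replication example actor that shows a changing value on a text render component.
; On BeginPlay, only the authority starts a looping one-second timer, which sets Variable to a random pick from the first three entries of the Variables array.
; The OnRep_Variable notify writes the new value to the text render, so the display follows the replicated variable without RPCs.
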(event Custom|PerSecond
  (Variables|Default|SetVariable (Utilities|Array|Get(acopy) (Variables|Default|GetVariables) (Math|Random|RandomIntegerinRange 0 2))))

(event EventBeginPlay
  (|CallParentFunction)
  (Networking|SwitchHasAuthority
    (:Authority
      (Utilities|Time|SetTimerbyEvent (delegate Custom|PerSecond) 1.0 true))))

(fn ConstructionScript
  (|CallParentFunction))

(fn OnRepVariable
  (Rendering|Components|TextRender|SetText (Variables|Default|GetTextRender) (Variables|Default|GetVariable)))