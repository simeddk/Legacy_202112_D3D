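; BP_CameraSplineTrigger is a trigger volume that starts and finishes progress on the camera actor as the player enters and leaves it.
; BeginPlay caches the player character as BP_CPlayer to filter overlaps on its Box.
; Begin overlap calls StartTimeline and end overlap calls OnFinishProgress on the first BP_CCameraActor found in the level through GetAllActorsOfClass.
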(event OnComponentBeginOverlap(Box)
  (params (OverlappedComponent :type Primitive%20Component%20Object%20Reference) (OtherActor :type Actor%20Object%20Reference) (OtherComp :type Primitive%20Component%20Object%20Reference) (OtherBodyIndex :type Integer) (bFromSweep :type Boolean) (SweepResult :type Hit%20Result%20Structure%20%28by%20ref%29))
  (if (== OtherActor (Variables|Default|GetPlayer))
    (bind _outactors (Actor|GetAllActorsOfClass "/Game/Cameras/BP_CCameraActor.BP_CCameraActor_C"))
    (Class|CCameraActor|StartTimeline (Utilities|Array|Get(acopy) _outactors))))

(event OnComponentEndOverlap(Box)
  (params (OverlappedComponent :type Primitive%20Component%20Object%20Reference) (OtherActor :type Actor%20Object%20Reference) (OtherComp :type Primitive%20Component%20Object%20Reference) (OtherBodyIndex :type Integer))
  (if (== OtherActor (Variables|Default|GetPlayer))
    (bind _outactors (Actor|GetAllActorsOfClass "/Game/Cameras/BP_CCameraActor.BP_CCameraActor_C"))
    (Class|CCameraActor|OnFinishProgress (Utilities|Array|Get(acopy) _outactors))))

(event EventBeginPlay
  (bind _asbp_cplayer (Utilities|Casting|CastToBP_CPlayer (Game|GetPlayerCharacter 0)))
  (Variables|Default|SetPlayer _asbp_cplayer))

(fn ConstructionScript)