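; BP_Robot is a mesh LOD demo actor that steps its static mesh through forced LOD levels and labels the current one.
; A looping one-second timer started on BeginPlay advances Index, wrapping to zero after four.
; Each tick of the timer passes Index to SetForcedLodModel and shows it as "LOD" plus that number on a TextRender component.
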(event Custom|PerSec
  (if (> (Variables|Default|GetIndex) 3)
    (Variables|Default|SetIndex 0)
    (else
      (Math|Integer|IncrementInt (Variables|Default|GetIndex)
        (:%20%20
          _))))
  (Rendering|LOD|SetForcedLodModel (Variables|Default|GetStaticMesh) (Variables|Default|GetIndex))
  (Rendering|Components|TextRender|SetText (Variables|Default|GetTextRender) (Utilities|Text|ToText(String) (Utilities|String|Append "LOD " (Utilities|String|ToString(Integer) (Variables|Default|GetIndex))))))

(event EventBeginPlay
  (Utilities|Time|SetTimerbyEvent (delegate Custom|PerSec) 1.0 true))

(fn ConstructionScript)